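; Motion warping manager component for the parkour system that plays parkour and simple montages warped to target points.
; Parkour moves cache up to four obstacle points, register them as warp targets, optionally play a camera animation, and notify the owning actor.
; A floor check at the landing point selects the default or fall montage section.
; A helper resizes the capsule per point, then restores it and the camera boom.
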(fn `PlayParkourAnimationWithItsSettings`
  (params (FirstPoint :type "Vector Structure") (SecondPoint :type "Vector Structure") (ThirdPoint :type "Vector Structure") (FourthPoint :type "Vector Structure") (AnimToPlay :type "/Game/ParkourSystem/Structs/AnimSettings/S_MW_AnimationSettings Structure") (SizeConfigForPoints :type "Array of /Game/ParkourSystem/Structs/AnimSettings/S_MW_SizeConfigs Structure") (SkeletalMeshComponent :type "SkeletalMeshComponent Object Reference") (CameraAnimHandle :type "CameraAnimationHandle Structure (by ref)") (ActorFrom :type "Actor Object Reference") (MotionWarpingComp :type "MotionWarpingComponent Object Reference") (PlayerController :type "PlayerController Object Reference"))
  (locals (L_Character :type "Character Object Reference"))
  (bind (_animationsettings_montagetoplay _animationsettings_cameraanimtoplay) (break `/Game/ParkourSystem/Structs/AnimSettings/S_MW_AnimationSettings` (`self.AnimationSettings`)))
  (bind (_animationsettings_montagetoplay_2 _animationsettings_cameraanimtoplay_2 _animationsettings_pointsforanimation _animationsettings_typeofaction) (break `/Game/ParkourSystem/Structs/AnimSettings/S_MW_AnimationSettings` (`self.AnimationSettings`)))
  (bind (_animationsettings_montagetoplay_3 _animationsettings_cameraanimtoplay_3) (break `/Game/ParkourSystem/Structs/AnimSettings/S_MW_AnimationSettings` (`self.AnimationSettings`)))
  (bind _m_sizeconfigforpoints (`self.m_SizeConfigForPoints`))
  (bind _animationsettings_montagetoplay_4 (break `/Game/ParkourSystem/Structs/AnimSettings/S_MW_AnimationSettings` (`self.AnimationSettings`)))
  (bind _animationsettings_montagetoplay_5 (break `/Game/ParkourSystem/Structs/AnimSettings/S_MW_AnimationSettings` (`self.AnimationSettings`)))
  (bind (_output_halfheightneeded _output_widthneeded) (break `/Game/ParkourSystem/Structs/AnimSettings/S_MW_SizeConfigs` (`|GetArrayItem` _m_sizeconfigforpoints (- (`KismetArrayLibrary.Array_Length` _m_sizeconfigforpoints) 1))))
  (set `self.AnimationSettings` AnimToPlay)
  (if (!= _animationsettings_montagetoplay_5 null)
    (set `self.m_FirstPoint` (`local.FirstPoint`))
    (set `self.m_SecondPoint` (`local.SecondPoint`))
    (set `self.m_ThirdPoint` (`local.ThirdPoint`))
    (set `self.m_FourthPoint` (`local.FourthPoint`))
    (set `self.ActorFrom` (`local.ActorFrom`))
    (set `self.m_SizeConfigForPoints` (`local.SizeConfigForPoints`))
    (bind _ascharacter (cast `Character` (`self.ActorFrom`)))
    (set `local.L_Character` _ascharacter)
    (`self.SetMotionWarpingComponentForParkourAnims` (`self.m_FirstPoint`) (`self.m_SecondPoint`) (`self.m_ThirdPoint`) (`self.m_FourthPoint`) MotionWarpingComp)
    (if (!= _animationsettings_cameraanimtoplay_3 null)
      (bind _returnvalue (`GameplayCamerasSubsystem.PlayCameraAnimation` (subsystem `GameplayCamerasSubsystem`) (`local.PlayerController`) _animationsettings_cameraanimtoplay (make `CameraAnimationParams` 1.0 1.0 "Linear" 0.2 "Linear" 0.3)))
      (`|VariableSetRef` (`local.CameraAnimHandle`) _returnvalue))
    (bind _returnvalue_2 (`/Game/ParkourSystem/ActorComponents/BFL_Helpers.FloorInPoint?` (`self.m_FourthPoint`) _output_widthneeded (`|MakeArray` "ObjectTypeQuery1" "ObjectTypeQuery2" :!type "EObjectTypeQuery Enum")))
    (if _returnvalue_2
      (`Character.PlayAnimMontage` (`local.L_Character`) _animationsettings_montagetoplay_4 1.0 "Default")
      (else
        (`Character.PlayAnimMontage` (`local.L_Character`) _animationsettings_montagetoplay_4 1.0 "DefToFall")))
    (`/Game/ParkourSystem/ActorComponents/BFL_Helpers.DrawObstaclePointsAndLandPoint` (`self.DrawDebug?`) (0.0 0.0 0.0) (`self.m_FirstPoint`) (`self.m_SecondPoint`) (`self.m_ThirdPoint`) (`self.m_FourthPoint`) 10.0 5.0 (struct :`R` 1.0 :`B` 0.783375 :`A` 1.0))
    (message `/Game/ParkourSystem/Interfaces/BI_MotionWarpingMessages.MotionWarpingStarted` (`self.ActorFrom`) _animationsettings_typeofaction)))

(fn `PlaySimpleAnimation`
  (params (PointToWarp :type "Vector Structure") (AnimToPlay :type "AnimMontage Object Reference") (MWComp :type "MotionWarpingComponent Object Reference") (Character :type "Character Object Reference") (WarpTargetRotation :type "Rotator Structure"))
  (set `self.ActorFrom` (`Actor.GetOwner` Character))
  (bind _output_get (set `self.m_FirstPoint` (`local.PointToWarp`)))
  (`self.SetMotionWarpingComponentForNormalAnims` _output_get MWComp WarpTargetRotation)
  (`Character.PlayAnimMontage` (`local.Character`) (`local.AnimToPlay`) 1.0 "Default")
  (message `/Game/ParkourSystem/Interfaces/BI_MotionWarpingMessages.MotionWarpingStarted` (`self.ActorFrom`) "NewEnumerator0"))

(fn `SetCapsuleToSizeConfig`
  (params (Index :type Integer) (CapsuleComponent :type "CapsuleComponent Object Reference") (InitWidth :type "Float (double-precision)") (InitHalfHeight :type "Float (double-precision)") (CameraBoom :type "SpringArmComponent Object Reference") (OrigCameraBoomLocation :type "Vector Structure"))
  (locals (L_CurrentSizeConfig :type "/Game/ParkourSystem/Structs/AnimSettings/S_MW_SizeConfigs Structure"))
  (bind (_l_currentsizeconfig_halfheightneeded _l_currentsizeconfig_widthneeded) (break `/Game/ParkourSystem/Structs/AnimSettings/S_MW_SizeConfigs` (`local.L_CurrentSizeConfig`)))
  (bind _l_currentsizeconfig_halfheightneeded_2 (break `/Game/ParkourSystem/Structs/AnimSettings/S_MW_SizeConfigs` (`local.L_CurrentSizeConfig`)))
  (bind _l_currentsizeconfig_halfheightneeded_3 (break `/Game/ParkourSystem/Structs/AnimSettings/S_MW_SizeConfigs` (`local.L_CurrentSizeConfig`)))
  (bind (_l_currentsizeconfig_halfheightneeded_4 _l_currentsizeconfig_widthneeded_2) (break `/Game/ParkourSystem/Structs/AnimSettings/S_MW_SizeConfigs` (`local.L_CurrentSizeConfig`)))
  (bind _cameraboom (`local.CameraBoom`))
  (bind (_l_currentsizeconfig_halfheightneeded_5 _l_currentsizeconfig_widthneeded_3) (break `/Game/ParkourSystem/Structs/AnimSettings/S_MW_SizeConfigs` (`local.L_CurrentSizeConfig`)))
  (bind (_l_currentsizeconfig_halfheightneeded_6 _l_currentsizeconfig_widthneeded_4) (break `/Game/ParkourSystem/Structs/AnimSettings/S_MW_SizeConfigs` (`local.L_CurrentSizeConfig`)))
  (if (< Index 4)
    (set `local.L_CurrentSizeConfig` (`|GetArrayItem` (`self.m_SizeConfigForPoints`) (`local.Index`)))
    (if (and (!= _l_currentsizeconfig_halfheightneeded 0.0) (!= _l_currentsizeconfig_widthneeded 0.0))
      (`CapsuleComponent.SetCapsuleSize` (`local.CapsuleComponent`) _l_currentsizeconfig_widthneeded_2 _l_currentsizeconfig_halfheightneeded_4 true)
      (else
        (if (!= _l_currentsizeconfig_halfheightneeded_2 0.0)
          (`CapsuleComponent.SetCapsuleHalfHeight` (`local.CapsuleComponent`) _l_currentsizeconfig_halfheightneeded_3 true))
        (if (!= _l_currentsizeconfig_widthneeded_3 0.0)
          (`CapsuleComponent.SetCapsuleRadius` (`local.CapsuleComponent`) _l_currentsizeconfig_widthneeded_4 true)
          (else
            (`CapsuleComponent.SetCapsuleRadius` (`local.CapsuleComponent`) (`local.InitWidth`) true)))))
    (else
      (`CapsuleComponent.SetCapsuleSize` (`local.CapsuleComponent`) InitWidth InitHalfHeight true)
      (`/Engine/EditorBlueprintResources/StandardMacros.IsValid` _cameraboom
        (:`Is Valid`
          (`SceneComponent.K2_SetRelativeLocation` _cameraboom (`local.OrigCameraBoomLocation`) false false))))))

(fn `SetMotionWarpingComponentForNormalAnims`
  (params (FirstPoint :type "Vector Structure") (MWComp :type "MotionWarpingComponent Object Reference") (`Warp Target Rotation` :type "Rotator Structure"))
  (`MotionWarpingComponent.AddOrUpdateWarpTarget` MWComp (make `MotionWarpingTarget` (`self.FirstPointName`) FirstPoint `Warp Target Rotation`)))

(fn `SetMotionWarpingComponentForParkourAnims`
  (params (FirstPoint :type "Vector Structure") (SecondPoint :type "Vector Structure") (ThirdPoint :type "Vector Structure") (FourthPoint :type "Vector Structure") (MWComponent :type "MotionWarpingComponent Object Reference"))
  (locals (L_CurrentIndex :type Integer))
  (bind (_animationsettings_montagetoplay _animationsettings_cameraanimtoplay _animationsettings_pointsforanimation) (break `/Game/ParkourSystem/Structs/AnimSettings/S_MW_AnimationSettings` (`self.AnimationSettings`)))
  (for (_ _array_index) _animationsettings_pointsforanimation
    (set `local.L_CurrentIndex` _array_index)
    (if (== (`local.L_CurrentIndex`) 0)
      (`MotionWarpingComponent.AddOrUpdateWarpTarget` (`local.MWComponent`) (make `MotionWarpingTarget` (`self.FirstPointName`) (`self.m_FirstPoint`) (`Actor.K2_GetActorRotation` (`self.ActorFrom`))))
      (elif (== (`local.L_CurrentIndex`) 1)
        (`MotionWarpingComponent.AddOrUpdateWarpTarget` (`local.MWComponent`) (make `MotionWarpingTarget` (`self.SecondPointName`) (`self.m_SecondPoint`) (`Actor.K2_GetActorRotation` (`self.ActorFrom`))))
        (elif (== (`local.L_CurrentIndex`) 2)
          (`MotionWarpingComponent.AddOrUpdateWarpTarget` (`local.MWComponent`) (make `MotionWarpingTarget` (`self.ThirdPointName`) (`self.m_ThirdPoint`) (`Actor.K2_GetActorRotation` (`self.ActorFrom`))))
          (elif (== (`local.L_CurrentIndex`) 3)
            (`MotionWarpingComponent.AddOrUpdateWarpTarget` (`local.MWComponent`) (make `MotionWarpingTarget` (`self.FourthPointName`) (`self.m_FourthPoint`) (`Actor.K2_GetActorRotation` (`self.ActorFrom`)))))))))
  (return))