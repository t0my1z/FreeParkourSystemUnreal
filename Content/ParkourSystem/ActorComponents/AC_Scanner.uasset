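; Parkour scanner component that detects obstacles ahead of an actor and returns them to the caller, intended for a filter component.
; A vertical stack of forward sphere traces gathers hit actors, skipping floors underfoot.
; Follow-up multi-sphere traces locate each one's start, base, end and middle points, from which height, width and distance are derived.
; Traces switch between object, channel or profile queries, and debug mode draws the points on Tick.
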(event `self.ReceiveTick`
  (params (DeltaSeconds :type "Float (single-precision)"))
  (if (and (> (`KismetArrayLibrary.Array_Length` (`self.ScannedObstacles`)) 0) (`self.DebugInformation`))
    (for _array_element (`self.ScannedObstacles`)
      (bind (_obstacleactor _obstacleheight _obstaclewidth _disttoobstacle _heighttoobstacle _basepoint _startpoint _middlepoint _endpoint) (break `/Game/ParkourSystem/Structs/Sensor/S_SC_Obstacle` _array_element))
      (`/Game/ParkourSystem/ActorComponents/BFL_Helpers.DrawObstaclePoints` _basepoint _startpoint _middlepoint _endpoint (`self.SphereRadius`) 0.0 (struct :`A` 1.0) (struct :`R` 0.095426 :`G` 1.0 :`A` 1.0) (struct :`G` 0.255931 :`B` 1.0 :`A` 1.0) (struct :`R` 1.0 :`A` 1.0)))))

(fn `DoesArrayOfHitsContainThisActor?`
  (params (HitArray :type "Array of HitResult Structure") (ActorToCheck :type "Actor Object Reference"))
  (returns (ReturnHit :type "HitResult Structure"))
  (locals (HitToReturn :type "HitResult Structure"))
  (for _array_element HitArray
    (bind (_bblockinghit _binitialoverlap _time _distance _location _impactpoint _normal _impactnormal _physmat _hitactor) (`GameplayStatics.BreakHitResult` _array_element))
    (if (and _bblockinghit (== _hitactor (`local.ActorToCheck`)))
      (set `local.HitToReturn` _array_element)
      (break)))
  (return (`local.HitToReturn`)))

(fn `DoMultiSphereTrace`
  (params (Start :type "Vector Structure") (End :type "Vector Structure") (`Override Type` :type Boolean) (`Type Of Coll` :type "/Game/ParkourSystem/Enums/E_TypeOfTrace Enum" :default "NewEnumerator0") (ActorsToIgnore :type "Array of Actor Object Reference"))
  (returns (OutHits :type "Array of HitResult Structure") (SuccesfullHit :type Boolean))
  (if `Override Type`
    (switch `/Game/ParkourSystem/Enums/E_TypeOfTrace` `Type Of Coll`
      (:`NewEnumerator0`
        _)
      (:`NewEnumerator1`
        (bind (_outhits _returnvalue) (`KismetSystemLibrary.SphereTraceMulti` (`local.Start`) (`local.End`) (`self.SphereRadius`) (`self.Trace Channel For Collisions`) false (`local.ActorsToIgnore`) (`self.Draw Debug Type`) :!label _label))
        (return _outhits _returnvalue))
      (:`NewEnumerator2`
        (bind (_outhits_2 _returnvalue_2) (`KismetSystemLibrary.SphereTraceMultiByProfile` (`local.Start`) (`local.End`) (`self.SphereRadius`) (`self.Profile Name For Collisions`) false (`local.ActorsToIgnore`) (`self.Draw Debug Type`) :!label _label_2))
        (return _outhits_2 _returnvalue_2)))
    (else
      (switch `/Game/ParkourSystem/Enums/E_TypeOfTrace` (`self.CurrentTypeofTrace`)
        (:`NewEnumerator0`
          _)
        (:`NewEnumerator1`
          (goto _label))
        (:`NewEnumerator2`
          (goto _label_2)))))
  (bind (_outhits_3 _returnvalue_3) (`KismetSystemLibrary.SphereTraceMultiForObjects` :`Start` (`local.Start`) :`End` (`local.End`) :`Radius` (`self.SphereRadius`) :`ObjectTypes` (`self.Object TypesToHit`) :`DrawDebugType` (`self.Draw Debug Type`)))
  (return _outhits_3 _returnvalue_3))

(fn `DoSingleSphereTrace`
  (params (Start :type "Vector Structure") (End :type "Vector Structure") (`Override Type` :type Boolean) (TypeOfCheck :type "/Game/ParkourSystem/Enums/E_TypeOfTrace Enum" :default "NewEnumerator0") (ActorsToIgnore :type "Array of Actor Object Reference"))
  (returns (OutHit :type "HitResult Structure") (SuccesfullHit :type Boolean))
  (if `Override Type`
    (switch `/Game/ParkourSystem/Enums/E_TypeOfTrace` TypeOfCheck
      (:`NewEnumerator0`
        _)
      (:`NewEnumerator1`
        (bind (_outhit _returnvalue) (`KismetSystemLibrary.SphereTraceSingle` (`local.Start`) (`local.End`) (`self.SphereRadius`) "TraceTypeQuery1" false (`local.ActorsToIgnore`) (`self.Draw Debug Type`) :!label _label))
        (return _outhit _returnvalue))
      (:`NewEnumerator2`
        (bind (_outhit_2 _returnvalue_2) (`KismetSystemLibrary.SphereTraceSingleByProfile` (`local.Start`) (`local.End`) (`self.SphereRadius`) (`self.Profile Name For Collisions`) false (`local.ActorsToIgnore`) (`self.Draw Debug Type`) :!label _label_2))
        (return _outhit_2 _returnvalue_2)))
    (else
      (switch `/Game/ParkourSystem/Enums/E_TypeOfTrace` (`self.CurrentTypeofTrace`)
        (:`NewEnumerator0`
          _)
        (:`NewEnumerator1`
          (goto _label))
        (:`NewEnumerator2`
          (goto _label_2)))))
  (bind (_outhit_3 _returnvalue_3) (`KismetSystemLibrary.SphereTraceSingleForObjects` (`local.Start`) (`local.End`) (`self.SphereRadius`) (`self.Object TypesToHit`) false (`local.ActorsToIgnore`) (`self.Draw Debug Type`)))
  (return _outhit_3 _returnvalue_3))

(fn `GetBasePointOfObstacle`
  (params (StartPointOfObstacle :type "Vector Structure") (`Contact Actor` :type "Actor Object Reference") (ActorsToIgnore :type "Array of Actor Object Reference"))
  (returns (BasePoint :type "Vector Structure"))
  (locals (L_HitObjects :type "Array of HitResult Structure") (TrueBasePoint :type "Vector Structure"))
  (bind (_actorlocation_x _actorlocation_y _actorlocation_z) (`KismetMathLibrary.BreakVector` (`self.ActorLocation`)))
  (bind _returnvalue (- _actorlocation_z (`self.HalfHeightOfCapsule`)))
  (bind (_startspherepoint _endspherepoint) (`/Game/ParkourSystem/ActorComponents/BFL_Helpers.DrawDebugSphereStartAndEnd` (- StartPointOfObstacle (* (`Actor.GetActorUpVector` (`self.ActorFrom`)) (`self.UpOffsetHeight`))) StartPointOfObstacle (`self.DebugTraceDuration`) (`self.SphereRadius`) (struct :`R` 0.0865 :`G` 0.955973 :`B` 0.896269 :`A` 1.0) (struct) (`self.DebugInformation`)))
  (bind (_outhits _succesfullhit) (`self.DoMultiSphereTrace` _startspherepoint _endspherepoint false "NewEnumerator0" (`local.ActorsToIgnore`)))
  (if _succesfullhit
    (bind _output_get (set `local.L_HitObjects` _outhits))
    (bind _returnhit (`self.DoesArrayOfHitsContainThisActor?` _output_get (`local.Contact Actor`)))
    (bind (_bblockinghit _binitialoverlap _time _distance _location _impactpoint) (`GameplayStatics.BreakHitResult` _returnhit))
    (if _bblockinghit
      (bind (_x _y _z) (`KismetMathLibrary.BreakVector3f` _impactpoint))
      (if (< _z _returnvalue)
        (bind _output_get_2 (set `local.TrueBasePoint` (`KismetMathLibrary.MakeVector` _x _y _returnvalue)))
        (return _output_get_2)
        (else
          (bind _output_get_3 (set `local.TrueBasePoint` _impactpoint))
          (return _output_get_3)))
      (else
        (return (0.0 0.0 0.0))))))

(fn `GetEndPointOfObstacle`
  (params (StartPointOfObstacle :type "Vector Structure") (ContactActor :type "Actor Object Reference") (ActorsToIgnore :type "Array of Actor Object Reference"))
  (returns (EndPoint :type "Vector Structure"))
  (locals (L_ForwardToBackHitObjects :type "Array of HitResult Structure") (L_UpHitObjects :type "Array of HitResult Structure") (EndPointLocatino :type "Vector Structure"))
  (bind _returnvalue (`Actor.GetActorUpVector` (`self.ActorFrom`)))
  (bind (_startspherepoint _endspherepoint) (`/Game/ParkourSystem/ActorComponents/BFL_Helpers.DrawDebugSphereStartAndEnd` (+ StartPointOfObstacle (* (`Actor.GetActorForwardVector` (`self.ActorFrom`)) (`self.ForwardOffsetWidth`))) StartPointOfObstacle (`self.DebugTraceDuration`) (`self.SphereRadius`) (struct :`R` 0.007499 :`G` 0.099899 :`B` 0.930111 :`A` 1.0) (struct :`R` 0.991102 :`G` 0.082283 :`B` 0.072272 :`A` 1.0) (`self.DebugInformation`)))
  (bind (_outhits _succesfullhit) (`self.DoMultiSphereTrace` _startspherepoint _endspherepoint false "NewEnumerator0" (`local.ActorsToIgnore`)))
  (if _succesfullhit
    (bind _output_get (set `local.L_ForwardToBackHitObjects` _outhits))
    (bind _returnhit (`self.DoesArrayOfHitsContainThisActor?` _output_get (`local.ContactActor`)))
    (bind (_bblockinghit _binitialoverlap _time _distance _location _impactpoint) (`GameplayStatics.BreakHitResult` _returnhit))
    (if _bblockinghit
      (bind (_startspherepoint_2 _endspherepoint_2) (`/Game/ParkourSystem/ActorComponents/BFL_Helpers.DrawDebugSphereStartAndEnd` (+ _impactpoint (* _returnvalue (`self.UpOffsetHeight`))) (+ _impactpoint (* _returnvalue -0.8)) (`self.DebugTraceDuration`) (`self.SphereRadius`) (struct :`R` 0.508881 :`G` 0.052861 :`B` 0.871367 :`A` 1.0) (struct :`G` 0.904661 :`B` 0.938686 :`A` 1.0) (`self.DebugInformation`)))
      (bind (_outhits_2 _succesfullhit_2) (`self.DoMultiSphereTrace` _startspherepoint_2 _endspherepoint_2 false "NewEnumerator0" (`local.ActorsToIgnore`)))
      (if _succesfullhit_2
        (bind _output_get_2 (set `local.L_UpHitObjects` _outhits_2))
        (bind _returnhit_2 (`self.DoesArrayOfHitsContainThisActor?` _output_get_2 (`local.ContactActor`)))
        (bind (_bblockinghit_2 _binitialoverlap_2 _time_2 _distance_2 _location_2 _impactpoint_2) (`GameplayStatics.BreakHitResult` _returnhit_2))
        (if _bblockinghit_2
          (return _impactpoint_2)
          (else
            (return (0.0 0.0 0.0))))))))

(fn `GetMiddlePointOfObstacle`
  (params (StartPointOfObstacle :type "Vector Structure") (EndPointOfObstacle :type "Vector Structure") (`Contact Actor` :type "Actor Object Reference") (ActorsToIgnore :type "Array of Actor Object Reference"))
  (returns (MiddlePoint :type "Vector Structure"))
  (locals (L_DistanceFromStartToEnd :type "Float (double-precision)" :default 0.0) (L_HitObjects :type "Array of HitResult Structure"))
  (bind _returnvalue (+ (`local.StartPointOfObstacle`) (* (`Actor.GetActorForwardVector` (`self.ActorFrom`)) (/ (`local.L_DistanceFromStartToEnd`) 2.0))))
  (set `local.L_DistanceFromStartToEnd` (`KismetMathLibrary.Vector_Distance` StartPointOfObstacle EndPointOfObstacle))
  (bind (_startspherepoint _endspherepoint) (`/Game/ParkourSystem/ActorComponents/BFL_Helpers.DrawDebugSphereStartAndEnd` (+ _returnvalue (* (`Actor.GetActorUpVector` (`self.ActorFrom`)) (`self.UpOffsetHeight`))) _returnvalue (`self.DebugTraceDuration`) (`self.SphereRadius`) (struct :`R` 1.0 :`G` 0.964686 :`B` 0.930111 :`A` 1.0) (struct :`R` 0.337164 :`B` 0.904661 :`A` 1.0) (`self.DebugInformation`)))
  (bind (_outhits _succesfullhit) (`self.DoMultiSphereTrace` _startspherepoint _endspherepoint false "NewEnumerator0" (`local.ActorsToIgnore`)))
  (if _succesfullhit
    (bind _output_get (set `local.L_HitObjects` _outhits))
    (bind _returnhit (`self.DoesArrayOfHitsContainThisActor?` _output_get (`local.Contact Actor`)))
    (bind (_bblockinghit _binitialoverlap _time _distance _location _impactpoint) (`GameplayStatics.BreakHitResult` _returnhit))
    (if _bblockinghit
      (return _impactpoint)
      (else
        (return (0.0 0.0 0.0))))))

(fn `GetObstacleInformation`
  (params (BasePointOfObstacle :type "Vector Structure") (StartPointOfObstacle :type "Vector Structure") (EndPointOfObstacle :type "Vector Structure") (MiddlePointOfObstacle :type "Vector Structure"))
  (returns (HeightOfObstacle :type "Float (double-precision)") (WidthOfObstacle :type "Float (double-precision)") (DistanceToObstacle :type "Float (double-precision)") (HeightToObstacle :type "Float (double-precision)"))
  (locals (L_HeightToObstacle :type "Float (double-precision)" :default 0.0) (L_HeightOfObstacle :type "Float (double-precision)" :default 0.0) (L_WidthOfObstacle :type "Float (double-precision)" :default 0.0) (L_DistanceToObstacle :type "Float (double-precision)" :default 0.0))
  (bind (_startpointofobstacle_x _startpointofobstacle_y _startpointofobstacle_z) (`KismetMathLibrary.BreakVector` (`local.StartPointOfObstacle`)))
  (bind (_actorlocation_x _actorlocation_y _actorlocation_z) (`KismetMathLibrary.BreakVector` (`self.ActorLocation`)))
  (bind (_actorlocation_x_2 _actorlocation_y_2) (`KismetMathLibrary.BreakVector` (`self.ActorLocation`)))
  (bind (_basepointofobstacle_x _basepointofobstacle_y) (`KismetMathLibrary.BreakVector` (`local.BasePointOfObstacle`)))
  (set `local.L_HeightToObstacle` (- _startpointofobstacle_z (- _actorlocation_z (`self.HalfHeightOfCapsule`))))
  (set `local.L_HeightOfObstacle` (`KismetMathLibrary.Vector_Distance` (`local.StartPointOfObstacle`) (`local.BasePointOfObstacle`)))
  (set `local.L_WidthOfObstacle` (`KismetMathLibrary.Vector_Distance` (`local.EndPointOfObstacle`) (`local.StartPointOfObstacle`)))
  (set `local.L_DistanceToObstacle` (`KismetMathLibrary.Distance2D` (`KismetMathLibrary.MakeVector2D` _basepointofobstacle_x _basepointofobstacle_y) (`KismetMathLibrary.MakeVector2D` _actorlocation_x_2 _actorlocation_y_2)))
  (return (`local.L_HeightOfObstacle`) (`local.L_WidthOfObstacle`) (`local.L_DistanceToObstacle`) (`local.L_HeightToObstacle`)))

(fn `GetStartPointOfObstacle`
  (params (ContactPoint :type "Vector Structure") (ContactActor :type "Actor Object Reference") (ActorsToIgnore :type "Array of Actor Object Reference"))
  (returns (StartPoint :type "Vector Structure"))
  (locals (L_HittedObjects :type "Array of HitResult Structure"))
  (bind (_outhits _succesfullhit) (`self.DoMultiSphereTrace` (+ ContactPoint (* (`Actor.GetActorUpVector` (`self.ActorFrom`)) (`self.UpOffsetHeight`))) ContactPoint false "NewEnumerator0" ActorsToIgnore))
  (if _succesfullhit
    (bind _output_get (set `local.L_HittedObjects` _outhits))
    (bind _returnhit (`self.DoesArrayOfHitsContainThisActor?` _output_get (`local.ContactActor`)))
    (bind (_bblockinghit _binitialoverlap _time _distance _location _impactpoint) (`GameplayStatics.BreakHitResult` _returnhit))
    (if _bblockinghit
      (return _impactpoint)
      (else
        (return (0.0 0.0 0.0))))))

(fn `HitInArrayContainsHitActor`
  (params (HitArray :type "Array of HitResult Structure") (HitToCheck :type "HitResult Structure"))
  (locals (L_HitResultNotContained :type Boolean) (L_CurrentArrayIndex :type Integer))
  (bind _hittocheck (`local.HitToCheck`))
  (bind _hittocheck_2 (`local.HitToCheck`))
  (if (> (`KismetArrayLibrary.Array_Length` HitArray) 0)
    (for (_array_element _array_index) (`local.HitArray`)
      (set `local.L_CurrentArrayIndex` _array_index)
      (if (!= (`.HitActor` (`GameplayStatics.BreakHitResult` _array_element)) (`.HitActor` (`GameplayStatics.BreakHitResult` (`local.HitToCheck`))))
        (set `local.L_HitResultNotContained` true)
        (else
          (`KismetArrayLibrary.Array_Set` (`local.HitArray`) (`local.L_CurrentArrayIndex`) (`local.HitToCheck`))
          (set `local.L_HitResultNotContained` false))))
    (if (`local.L_HitResultNotContained`)
      (`KismetArrayLibrary.Array_Add` (`local.HitArray`) _hittocheck_2)
      (if (`self.DebugInformation`)
        (`KismetSystemLibrary.PrintString` (`KismetSystemLibrary.GetDisplayName` (`.HitActor` (`GameplayStatics.BreakHitResult` _hittocheck_2))) true true (struct :`R` 1.0 :`G` 0.078022 :`B` 0.96813 :`A` 1.0) (`self.DebugTraceDuration`))
        (return)
        (else
          (return))))
    (else
      (`KismetArrayLibrary.Array_Add` (`local.HitArray`) _hittocheck)
      (if (`self.DebugInformation`)
        (`KismetSystemLibrary.PrintString` (`KismetSystemLibrary.GetDisplayName` (`.HitActor` (`GameplayStatics.BreakHitResult` _hittocheck))) true true (struct :`R` 0.045849 :`G` 1.0 :`B` 0.025666 :`A` 1.0) (`self.DebugTraceDuration`))
        (return)
        (else
          (return))))))

(fn `Scan Enviroment`
  (params (ActorReceived :type "Actor Object Reference") (HalfHeightOfActor :type "Float (double-precision)"))
  (returns (ScannedObstacles :type "Array of /Game/ParkourSystem/Structs/Sensor/S_SC_Obstacle Structure"))
  (locals (L_HitResults :type "Array of HitResult Structure") (L_HitActors :type "Array of Actor Object Reference") (L_ActorsToIgnore :type "Array of Actor Object Reference"))
  (`|ExecutionSequence`
    (:`then_0`
      ;[1 0.8122 0.108] CG To Set Our Variables for the Scan
      (bind _output_get (set `self.ActorFrom` (`local.ActorReceived`)))
      (set `self.ActorLocation` (`Actor.K2_GetActorLocation` _output_get))
      (`KismetArrayLibrary.Array_Clear` (`local.L_HitResults`))
      (`KismetArrayLibrary.Array_Clear` (`self.ScannedObstacles`))
      (set `self.HalfHeightOfCapsule` (`local.HalfHeightOfActor`)))
    (:`then_1`
      ;[1 0.1456 0.7864] CG in which we launch forward sphere traces with a height offset between them in a loop with the number of loops we pass on
      (bind _hittedactors (`/Game/ParkourSystem/ActorComponents/BFL_Helpers.GetAllFloorsUnder` (`self.ActorFrom`) (`self.SphereRadius`) (`self.DownOffsetForForwardTraces`) (`self.Object TypesToHit`)))
      (set `local.L_ActorsToIgnore` _hittedactors)
      (for _index (range (+ (`self.NumberOfForwardSpehreCasts`) 1))
        (bind _returnvalue (+ (- (`self.ActorLocation`) (`KismetMathLibrary.MakeVector` 0.0 0.0 (`self.DownOffsetForForwardTraces`))) (`KismetMathLibrary.MakeVector` 0.0 0.0 (* _index (`self.UpOffsetBetweenForwardTraces`)))))
        (bind (_outhit _succesfullhit) (`self.DoSingleSphereTrace` _returnvalue (+ _returnvalue (* (`Actor.GetActorForwardVector` (`self.ActorFrom`)) (`self.ForwardDistanceOfTraces`))) false "NewEnumerator0" (`local.L_ActorsToIgnore`)))
        (if _succesfullhit
          (`self.HitInArrayContainsHitActor` (`local.L_HitResults`) _outhit))))
    (:`then_2`
      ;[0.07743 0.9003 1] CG in which we loop through our HitResults and create Obstacles, set all their corresponding variables, and then add them to our ScannedObstacles list
      (if (> (`KismetArrayLibrary.Array_Length` (`local.L_HitResults`)) 0)
        (for _array_element (`local.L_HitResults`)
          (`KismetArrayLibrary.Array_Add` (`local.L_HitActors`) (`.HitActor` (`GameplayStatics.BreakHitResult` _array_element))))
        (bind _outactors (`/Game/ParkourSystem/ActorComponents/BFL_Helpers.GetFloorsUnder` (`self.ActorFrom`) (`self.HalfHeightOfCapsule`) (`self.SphereRadius`) (`self.Object TypesToHit`)))
        (for _array_element_2 _outactors
          (`KismetArrayLibrary.Array_Add` (`local.L_HitActors`) _array_element_2))
        (`self.SetObstacleFromHitResult` (`local.L_HitResults`) (`local.L_HitActors`))))
    (:`then_3`
      ;[0.2433 1 0.07432] Pass Our Scanned Obstacles To The One Calling This Function, since be Expect them to use the Filter Component to filter them
      (return (`self.ScannedObstacles`)))))

(fn `SetObstacleAndIt`
  (params (HittedActir :type "Actor Object Reference") (ObstacleHeight :type "Float (double-precision)") (ObstacleWidth :type "Float (double-precision)") (DistToObstacle :type "Float (double-precision)") (HeightToObstacle :type "Float (double-precision)") (BasePoint :type "Vector Structure") (StartPoint :type "Vector Structure") (MiddlePoint :type "Vector Structure") (EndPoint :type "Vector Structure"))
  (locals (L_NewObstacle :type "/Game/ParkourSystem/Structs/Sensor/S_SC_Obstacle Structure"))
  (bind _output_get (set `local.L_NewObstacle` (make `/Game/ParkourSystem/Structs/Sensor/S_SC_Obstacle` HittedActir ObstacleHeight ObstacleWidth DistToObstacle HeightToObstacle BasePoint StartPoint MiddlePoint EndPoint)))
  (`KismetArrayLibrary.Array_Add` (`self.ScannedObstacles`) _output_get)
  (if (not (`self.DebugInformation`))
    (return)
    (else
      (`KismetSystemLibrary.PrintString` "Im Adding an Obstacle" true true (struct :`G` 0.66 :`B` 1.0 :`A` 1.0) (`self.DebugTraceDuration`))
      (return))))

(fn `SetObstacleFromHitResult`
  (params (HitResults :type "Array of HitResult Structure") (AllActorsDetected :type "Array of Actor Object Reference"))
  (locals (L_HittedActor :type "Actor Object Reference") (L_ActorsToIgnore :type "Array of Actor Object Reference") (L_ContactPointLocation :type "Vector Structure" :default (0.0 0.0 0.0)) (L_ObstacleHeight :type "Float (double-precision)") (L_ObstacleWidth :type "Float (double-precision)") (L_DistToObstacle :type "Float (double-precision)") (L_HeightToObstacle :type "Float (double-precision)") (L_BasePointOfObstacle :type "Vector Structure") (L_StartPointOfObstacle :type "Vector Structure") (L_MiddlePointOfObstacle :type "Vector Structure") (L_EndPointOfObstacle :type "Vector Structure"))
  (for _array_element HitResults
    (set `local.L_ActorsToIgnore` (`local.AllActorsDetected`))
    (bind (_bblockinghit _binitialoverlap _time _distance _location _impactpoint _normal _impactnormal _physmat _hitactor) (`GameplayStatics.BreakHitResult` _array_element))
    (bind _returnvalue (`KismetArrayLibrary.Array_RemoveItem` (`local.L_ActorsToIgnore`) _hitactor))
    (if _returnvalue
      (bind _output_get (set `local.L_HittedActor` _hitactor))
      (if (`self.DebugInformation`)
        (`KismetSystemLibrary.PrintString` (`KismetSystemLibrary.GetDisplayName` _output_get) true true (struct :`R` 0.519096 :`B` 1.0 :`A` 1.0) (`self.DebugTraceDuration`)))
      (set `local.L_ContactPointLocation` _impactpoint)
      (`|ExecutionSequence`
        (:`then_0`
          (bind _startpoint (`self.GetStartPointOfObstacle` (`local.L_ContactPointLocation`) (`local.L_HittedActor`) (`local.L_ActorsToIgnore`)))
          (set `local.L_StartPointOfObstacle` _startpoint))
        (:`then_1`
          (bind _basepoint (`self.GetBasePointOfObstacle` (`local.L_StartPointOfObstacle`) (`local.L_HittedActor`) (`local.L_ActorsToIgnore`)))
          (set `local.L_BasePointOfObstacle` _basepoint))
        (:`then_2`
          (bind _endpoint (`self.GetEndPointOfObstacle` (`local.L_StartPointOfObstacle`) (`local.L_HittedActor`) (`local.L_ActorsToIgnore`)))
          (set `local.L_EndPointOfObstacle` _endpoint))
        (:`then_3`
          (bind _middlepoint (`self.GetMiddlePointOfObstacle` (`local.L_StartPointOfObstacle`) (`local.L_EndPointOfObstacle`) (`local.L_HittedActor`) (`local.L_ActorsToIgnore`)))
          (set `local.L_MiddlePointOfObstacle` _middlepoint))
        (:`then_4`
          (bind (_heightofobstacle _widthofobstacle _distancetoobstacle _heighttoobstacle) (`self.GetObstacleInformation` (`local.L_BasePointOfObstacle`) (`local.L_StartPointOfObstacle`) (`local.L_EndPointOfObstacle`) (`local.L_MiddlePointOfObstacle`)))
          (set `local.L_ObstacleHeight` _heightofobstacle)
          (set `local.L_ObstacleWidth` _widthofobstacle)
          (set `local.L_DistToObstacle` _distancetoobstacle)
          (set `local.L_HeightToObstacle` _heighttoobstacle))
        (:`then_5`
          (`self.SetObstacleAndIt` (`local.L_HittedActor`) (`local.L_ObstacleHeight`) (`local.L_ObstacleWidth`) (`local.L_DistToObstacle`) (`local.L_HeightToObstacle`) (`local.L_BasePointOfObstacle`) (`local.L_StartPointOfObstacle`) (`local.L_MiddlePointOfObstacle`) (`local.L_EndPointOfObstacle`)))))))